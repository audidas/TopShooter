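; Master Blueprint for building structures that lets their meshes fade through a material opacity parameter.
; BeginPlay creates dynamic material instances for every static mesh component material, skipping components tagged IgnoreFade, and caches them in a list.
; SetFadeOpacity reference-counts fade requests, so only the first request applies the faded value and opacity is restored once the count drops to zero or below.
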(event `self.ReceiveBeginPlay`
  (for _array_element (`self.K2_GetComponentsByClass` "/Script/Engine.StaticMeshComponent")
    (if (not (`ActorComponent.ComponentHasTag` _array_element "IgnoreFade"))
      (for _index (range (`PrimitiveComponent.GetNumMaterials` _array_element))
        (bind _returnvalue (`PrimitiveComponent.CreateDynamicMaterialInstance` _array_element _index null "None"))
        (`KismetArrayLibrary.Array_Add` (`self.DMI_List`) _returnvalue)))))

(event `OCFadeInterface.SetFadeOpacity`
  (params (Opacity :type "Float (single-precision)"))
  (if (< Opacity 1.0)
    (bind _result (`/Engine/EditorBlueprintResources/StandardMacros.IncrementInt` (`self.TriggerCount`))
      (:`  `
        (if (== _result 1)
          (for _array_element (`self.DMI_List`)
            (`MaterialInstanceDynamic.SetScalarParameterValue` _array_element "FadeOpacity" Opacity)))))
    (else
      (bind _result_2 (`/Engine/EditorBlueprintResources/StandardMacros.DecrementInt` (`self.TriggerCount`))
        (:`  `
          (if (== (`KismetMathLibrary.Clamp` _result_2 0 1) 0)
            (for _array_element_2 (`self.DMI_List`)
              (`MaterialInstanceDynamic.SetScalarParameterValue` _array_element_2 "FadeOpacity" Opacity))))))))

(fn `UserConstructionScript`)