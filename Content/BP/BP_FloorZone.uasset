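; BP_FloorZone is a trigger zone that swaps the fade opacity of two object lists as the player enters or leaves its Box.
; On overlap by an actor tagged Player, it messages HideList to fade to zero and ShowList to full opacity, reversing both on exit.
; The ShowList loop is nested inside the HideList loop, so it repeats per hidden element and never runs when HideList is empty.
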(event `self.Box.OnComponentBeginOverlap`
  (params (OverlappedComponent :type "PrimitiveComponent Object Reference") (OtherActor :type "Actor Object Reference") (OtherComp :type "PrimitiveComponent Object Reference") (OtherBodyIndex :type Integer) (bFromSweep :type Boolean) (SweepResult :type "HitResult Structure (by ref)"))
  (if (`self.ActorHasTag` OtherActor "Player")
    (for _array_element (`self.HideList`)
      (message `OCFadeInterface.SetFadeOpacity` _array_element 0.0)
      (for _array_element_2 (`self.ShowList`)
        (message `OCFadeInterface.SetFadeOpacity` _array_element_2 1.0)))))

(event `self.Box.OnComponentEndOverlap`
  (params (OverlappedComponent :type "PrimitiveComponent Object Reference") (OtherActor :type "Actor Object Reference") (OtherComp :type "PrimitiveComponent Object Reference") (OtherBodyIndex :type Integer))
  (if (`self.ActorHasTag` OtherActor "Player")
    (for _array_element (`self.HideList`)
      (message `OCFadeInterface.SetFadeOpacity` _array_element 1.0)
      (for _array_element_2 (`self.ShowList`)
        (message `OCFadeInterface.SetFadeOpacity` _array_element_2 0.0)))))

(fn `UserConstructionScript`)